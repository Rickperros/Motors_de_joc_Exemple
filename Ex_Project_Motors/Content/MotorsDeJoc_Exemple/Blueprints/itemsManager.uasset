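; Items manager actor that keeps count of the keys and coins picked up in the game.
; ItemPicked takes a collectable type, increments the matching count in a string-keyed Items map, then fires the ItemManagerStatusChanged dispatcher to announce the change.
; As a debug readout, it also writes both totals to the CoinsRender and KeysRender text components.
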(fn ConstructionScript)

(fn ItemPicked
  (params (Collactable :type ECollactableType%20Enum :default "NewEnumerator0"))
  (bind _items (Variables|Default|GetItems))
  (Utilities|FlowControl|Sequence
    (:then_0
      (switch Utilities|FlowControl|Switch|SwitchonECollactableType Collactable
        (:NewEnumerator0
          (bind _result (Math|Integer|IncrementInt (.Value (Utilities|Map|Find (Variables|Default|GetItems) "Keys")))
            (:%20%20
              (Utilities|Map|Add (Variables|Default|GetItems) "Keys" _result))))
        (:NewEnumerator1
          (bind _result_2 (Math|Integer|IncrementInt (.Value (Utilities|Map|Find (Variables|Default|GetItems) "Coins")))
            (:%20%20
              (Utilities|Map|Add (Variables|Default|GetItems) "Coins" _result_2))))))
    (:then_1
      (Default|CallItemManagerStatusChanged))
    (:then_2
      ;[1 0.82 0] DEBUG
      (Rendering|Components|TextRender|SetText (Variables|Default|GetCoinsRender) (Utilities|Text|ToText(String) (Utilities|String|Append "Coins: " (Utilities|String|ToString(Integer) (.Value (Utilities|Map|Find _items "Coins"))))))
      (Rendering|Components|TextRender|SetText (Variables|Default|GetKeysRender) (Utilities|Text|ToText(String) (Utilities|String|Append "Keys: " (Utilities|String|ToString(Integer) (.Value (Utilities|Map|Find _items "Keys")))))))))