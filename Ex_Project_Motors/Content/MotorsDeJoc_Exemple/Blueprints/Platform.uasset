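; Platform actor whose mesh dissolves away and back when the 5 key is pressed.
; On BeginPlay it creates a dynamic material instance from the mesh's first material and applies it to that slot.
; Alternate presses play or reverse a timeline that drives the DisolutionVal scalar parameter, with AllowBurn enabled on the forward press.
; Only material parameters change; the Blueprint does not touch collision or visibility.
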(event EventBeginPlay
  (bind _staticmesh (Variables|Default|GetStaticMesh))
  (bind _returnvalue (Rendering|Material|CreateDynamicMaterialInstance (Utilities|Array|Get(acopy) (Rendering|Material|GetMaterials _staticmesh)) "DisolutionMat_DInst" :!class /Script/Engine.KismetMaterialLibrary))
  (Rendering|Material|SetMaterial _staticmesh 0 _returnvalue))

(event Input|KeyboardEvents|5
  (params (Key :type Key%20Structure :default "None"))
  (bind _staticmesh (Variables|Default|GetStaticMesh))
  (:Pressed
    (Utilities|FlowControl|FlipFlop
      (:A
        (Rendering|Material|SetScalarParameterValueonMaterials _staticmesh "AllowBurn" 1.0)
        (bind _disolutionvalue (Timeline|DisolutionTimeline Play)
          (:Update
            (Rendering|Material|SetScalarParameterValueonMaterials _staticmesh "DisolutionVal" _disolutionvalue))))
      (:B
        (Timeline|DisolutionTimeline Reverse)))))

(fn ConstructionScript)