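; HUDManager shows the collectable items tracked by the level's ItemsManager on the player's screen.
; On BeginPlay it finds the first ItemsManager actor, lazily creates the PlayerHUD widget and adds it to the viewport.
; It binds to the manager's status-changed dispatcher and passes the current Items to the widget, both at start and on each change.
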(event Custom|ItemManager_StatusChanged
  (Default|AddTextonScreen (Variables|Default|GetCollactable_HUD) (Variables|/Game/MotorsDeJoc_Exemple/Blueprints/itemsManager.ItemsManager_C|GetItems (Variables|Default|GetItemManager))))

(event EventBeginPlay
  (CallFunction|SetItemManager)
  (EventDispatchers|AssignItemManagerStatusChanged (Variables|Default|GetItemManager) (delegate Custom|ItemManager_StatusChanged))
  ;[0 1 0.006319] Add Player HUD to screen
  (UserInterface|Viewport|AddtoViewport (CallFunction|GetCollactableHUD) 0)
  (Default|AddTextonScreen (Variables|Default|GetCollactable_HUD) (Variables|/Game/MotorsDeJoc_Exemple/Blueprints/itemsManager.ItemsManager_C|GetItems (Variables|Default|GetItemManager))))

(fn ConstructionScript)

(fn GetCollactableHUD
  (Variables|Default|GetCollactable_HUD
    (:then
      _)
    (:else
      (bind _returnvalue (UserInterface|CreateWidget "/Game/MotorsDeJoc_Exemple/Blueprints/PlayerHUD.PlayerHUD_C"))
      (Variables|Default|SetCollactable_HUD _returnvalue)))
  (return (Variables|Default|GetCollactable_HUD)))

(fn SetItemManager
  (bind _outactors (Actor|GetAllActorsOfClass "/Game/MotorsDeJoc_Exemple/Blueprints/itemsManager.ItemsManager_C"))
  (Variables|Default|SetItemManager (Utilities|Array|Get(acopy) _outactors)))